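; BP_Cart is the player paddle, moved sideways by MoveRight with swept offsets, that manages balls and lives.
; It spawns up to three BP_Balls and binds their OnDead, costing HP when none remain, then respawning or signaling game end.
; Overlapped BP_Bonus pickups add a ball or life, remove a ball, or resize the paddle.
; A retriggerable delay restores default length, and growing near an edge first nudges the paddle inward.
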(event `self.ReceiveBeginPlay`
  (set `self.DefaultLenght` (`self.GetActorScale3D`))
  (`self.Spawn Ball`))

(event `InputAxis|MoveRight`
  (params (AxisValue :type "Float (single-precision)"))
  (if (< AxisValue 0.0)
    (`self.K2_AddActorWorldOffset` (0.0 -10.0 0.0) true)))

(event `InputAxis|MoveRight`
  (params (AxisValue :type "Float (single-precision)"))
  (if (> AxisValue 0.0)
    (`self.K2_AddActorWorldOffset` (0.0 10.0 0.0) true)))

(event `Spawn Ball`
  (if (< (`self.CountBall`) 3)
    (bind _returnvalue (`|SpawnActorFromClass` "/Game/MyGame/BluePrints/BP_Ball.BP_Ball_C" (`KismetMathLibrary.MakeTransform` (`SceneComponent.K2_GetComponentLocation` (`self.Sphere`))) "AlwaysSpawn" "OverrideRootScale" null null))
    (bind _output_get (set `self.PlayingBall` _returnvalue))
    (add `/Game/MyGame/BluePrints/BP_Ball.OnDead` _output_get (delegate `DeadBall`))
    (bind _result (`/Engine/EditorBlueprintResources/StandardMacros.IncrementInt` (`self.CountBall`))
      (:`  `
        (set `self.CountBall` _result)))))

(event `DeadBall`
  (bind _result (`/Engine/EditorBlueprintResources/StandardMacros.DecrementInt` (`self.CountBall`))
    (:`  `
      (if (<= _result 0)
        (bind _result_2 (`/Engine/EditorBlueprintResources/StandardMacros.DecrementInt` (`self.HP`))
          (:`  `
            (`GameplayStatics.SpawnSound2D` "/Game/MyGame/Sounds/Die_Cue.Die_Cue" 1.0 1.0 0.0 null)
            (`self.LivesChanged` _result_2)
            (if (> _result_2 0)
              (if (== (`self.CountBall`) 0) :!label _label
                (`self.Spawn Ball`))
              (else
                (`GameplayStatics.SpawnSound2D` "/Game/MyGame/Sounds/Sound_Lose_Cue.Sound_Lose_Cue" 1.0 1.0 0.0 null)
                (`self.GameEnd`)))))
        (else
          (goto _label))))))

(event `TimerForReduceLenght`
  (`KismetSystemLibrary.RetriggerableDelay` 10.0)
  (`self.SetActorScale3D` (`self.DefaultLenght`)))

(event `self.ReceiveActorBeginOverlap`
  (params (OtherActor :type "Actor Object Reference"))
  (bind _bonusball (`self.BonusBall`))
  (bind _asbp_bonus (cast `/Game/MyGame/BluePrints/Bonuses/BP_Bonus` OtherActor))
  (set `self.BonusBall` _asbp_bonus)
  (if (`/Game/MyGame/BluePrints/Bonuses/BP_Bonus.BonusBall` _bonusball)
    (`self.Spawn Ball`)
    (`GameplayStatics.PlaySoundAtLocation` "/Game/MyGame/Sounds/Sound_Bonus_Cue.Sound_Bonus_Cue" (`self.K2_GetActorLocation`) (struct) 1.0 1.0 0.0 null null null :!label _label_2)
    (`self.K2_DestroyActor` (`self.BonusBall`))
    (elif (`/Game/MyGame/BluePrints/Bonuses/BP_Bonus.BonusHP` _bonusball)
      (bind _result (`/Engine/EditorBlueprintResources/StandardMacros.IncrementInt` (`self.HP`))
        (:`  `
          (`self.LivesChanged` _result)
          (goto _label_2)))
      (elif (`/Game/MyGame/BluePrints/Bonuses/BP_Bonus.BonusMaxLenght` _bonusball)
        (`self.Increasing the lenght`)
        (`self.TimerForReduceLenght`)
        (goto _label_2)
        (elif (`/Game/MyGame/BluePrints/Bonuses/BP_Bonus.DebuffMinLenght` _bonusball)
          (`self.Reducing the lenght`)
          (`self.TimerForReduceLenght`)
          (goto _label_2)
          (elif (`/Game/MyGame/BluePrints/Bonuses/BP_Bonus.MinusBall` _bonusball)
            (if (> (`self.CountBall`) 1)
              (add `self.OnActorBeginOverlap` (delegate `DestroyPlayingBall`)))))))))

(event `DestroyPlayingBall` :!signature `self.OnActorBeginOverlap`
  (params (OverlappedActor :type "Actor Object Reference") (OtherActor :type "Actor Object Reference"))
  (cast `/Game/MyGame/BluePrints/Bonuses/BP_MinusBall` OtherActor)
  (bind _result (`/Engine/EditorBlueprintResources/StandardMacros.DecrementInt` (`self.CountBall`))
    (:`  `
      (set `self.CountBall` _result)
      (`self.K2_DestroyActor` (`self.PlayingBall`))
      (goto _label_2))))

(fn `Increasing the lenght`
  (bind (_returnvalue_x _returnvalue_y _returnvalue_z) (`KismetMathLibrary.BreakVector` (`self.GetActorScale3D`)))
  (bind (_returnvalue_x_2 _returnvalue_y_2 _returnvalue_z_2) (`KismetMathLibrary.BreakVector` (`self.K2_GetActorLocation`)))
  (bind (_returnvalue_x_3 _returnvalue_y_3) (`KismetMathLibrary.BreakVector` (`self.K2_GetActorLocation`)))
  (bind _maxlenght (`self.MaxLenght`))
  (bind _returnvalue (* _returnvalue_y 1.5))
  (if (>= (`KismetMathLibrary.Abs` _returnvalue_y_3) 500.0)
    (`self.K2_SetActorLocation` (`KismetMathLibrary.MakeVector` _returnvalue_x_2 (+ _returnvalue_y_2 (`KismetMathLibrary.SelectFloat` -100.0 100.0 (> _returnvalue_y_2 0.0))) _returnvalue_z_2)))
  (if (<= _returnvalue _maxlenght)
    (`self.SetActorScale3D` (`KismetMathLibrary.MakeVector` _returnvalue_x _returnvalue _returnvalue_z))
    (else
      (`self.SetActorScale3D` (`KismetMathLibrary.MakeVector` _returnvalue_x _maxlenght _returnvalue_z)))))

(fn `Reducing the lenght`
  (bind (_returnvalue_x _returnvalue_y _returnvalue_z) (`KismetMathLibrary.BreakVector` (`self.GetActorScale3D`)))
  (bind _returnvalue (* _returnvalue_y 0.8))
  (if (>= _returnvalue (`self.MinLenght`))
    (`self.SetActorScale3D` (`KismetMathLibrary.MakeVector` _returnvalue_x _returnvalue _returnvalue_z))
    (else
      (`self.SetActorScale3D` (`KismetMathLibrary.MakeVector` _returnvalue_x 0.0 _returnvalue_z)))))

(fn `UserConstructionScript`
  (`SceneComponent.SetWorldScale3D` (`self.Cube`) (0.25 5.0 1.0)))