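; Player controller that runs the HUD, win/lose screen and exit to menu for a level.
; BeginPlay creates the HUD and binds the cube generator's all-cubes-died event to a win, while possessing a BP_Cart binds its game-end event to a loss.
; Both outcomes share one path that hides the HUD, shows the result widget and switches to UI-only input with a cursor.
; The Exit input opens the Menu level.
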(event `self.ReceiveBeginPlay`
  (`|ExecutionSequence`
    (:`then_0`
      (`WidgetBlueprintLibrary.SetInputMode_GameOnly` self)
      (bind _returnvalue (`|CreateWidget` "/Game/MyGame/UI/WBP_HUD.WBP_HUD_C" self))
      (`UserWidget.AddToViewport` _returnvalue 0)
      (set `self.HUD` _returnvalue))
    (:`then_1`
      (bind _returnvalue_2 (`GameplayStatics.GetActorOfClass` "/Game/MyGame/BluePrints/Core/BP_CubeGenerator.BP_CubeGenerator_C"))
      (add `/Game/MyGame/BluePrints/Core/BP_CubeGenerator.AllCubesDied` _returnvalue_2 (delegate `GameFinished`)))))

(event `GameFinished`
  (bind _hud (`self.HUD`))
  (set `self.IsWinner` true)
  (`/Engine/EditorBlueprintResources/StandardMacros.IsValid` _hud
    (:`Is Valid`
      (`Widget.SetVisibility` _hud "Collapsed" :!label _label)
      (bind _returnvalue (`|CreateWidget` "/Game/MyGame/UI/WBP_WINSCREEN.WBP_WINSCREEN_C" self))
      (`/Game/MyGame/UI/WBP_WINSCREEN.UpdateWinner` _returnvalue (`self.IsWinner`))
      (`UserWidget.AddToViewport` _returnvalue 0)
      (`WidgetBlueprintLibrary.SetInputMode_UIOnlyEx` self _returnvalue "LockOnCapture")
      (set `self.bShowMouseCursor` true))))

(event `PlayerLose`
  (set `self.IsWinner` false)
  (`/Engine/EditorBlueprintResources/StandardMacros.IsValid` (`self.HUD`)
    (:`Is Valid`
      (goto _label))))

(event `self.ReceivePossess`
  (params (PossessedPawn :type "Pawn Object Reference"))
  (bind _asbp_cart (cast `/Game/MyGame/BluePrints/BP_Cart` PossessedPawn))
  (bind _output_get (set `self.My Cart` _asbp_cart))
  (add `/Game/MyGame/BluePrints/BP_Cart.GameEnd` _output_get (delegate `PlayerLose`)))

(event `InputAction|Exit`
  (params (Key :type "Key Structure"))
  (:`Pressed`
    (`GameplayStatics.OpenLevelBySoftObjectPtr` "/Game/MyGame/Maps/Menu.Menu")))

(fn `UserConstructionScript`)