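; Actor that builds an X by Y grid of BP_Cube_Child actors and tracks score and win state as they die.
; The construction script previews the grid with static mesh components, which BeginPlay destroys before spawning the real cubes at padded offsets from its location.
; It binds each cube's death event, adds absolute scores and broadcasts the total.
; When all cubes are dead, it plays a winner sound and fires AllCubesDied.
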(event `self.ReceiveBeginPlay`
  (bind (_returnvalue_x _returnvalue_y _returnvalue_z) (`KismetMathLibrary.BreakVector` (`self.K2_GetActorLocation`)))
  (for _array_element (`self.PreviewArray`)
    (`ActorComponent.K2_DestroyComponent` _array_element))
  (for _index (range (+ (`self.X`) 1))
    (for _index_2 (range (+ (`self.Y`) 1))
      (bind _returnvalue (`|SpawnActorFromClass` "/Game/MyGame/BluePrints/BP_Cube_Child.BP_Cube_Child_C" (`KismetMathLibrary.MakeTransform` (`KismetMathLibrary.MakeVector` (+ (`KismetMathLibrary.Conv_IntToDouble` (* _index (`self.Padding`))) _returnvalue_x) (+ (`KismetMathLibrary.Conv_IntToDouble` (* _index_2 (`self.Padding`))) _returnvalue_y) _returnvalue_z)) "Undefined" "OverrideRootScale" null null))
      (`KismetArrayLibrary.Array_Add` (`self.CubeArray`) _returnvalue)))
  (bind _amountcubes (`self.GetCubesFoWin`))
  (set `self.AmountCubesForWin` _amountcubes)
  (for _array_element_2 (`self.CubeArray`)
    (add `/Game/MyGame/BluePrints/BP_Cube_Parent.CubeDead` _array_element_2 (delegate `CubeDestroyed`))))

(event `CubeDestroyed`
  (params (Score :type Integer))
  (bind _amount_score (`self.AddedScore` Score))
  (`self.ScoreChanged` _amount_score)
  (`/Engine/EditorBlueprintResources/StandardMacros.IncrementInt` (`self.CountDeadCubes`)
    (:`  `
      (if (>= (`self.CountDeadCubes`) (`self.AmountCubesForWin`))
        (`GameplayStatics.PlaySound2D` "/Game/MyGame/Sounds/Sound_Winner_Cue.Sound_Winner_Cue" 1.0 1.0 0.0 null null)
        (`self.AllCubesDied`)))))

(fn `AddedScore`
  (params (Score :type Integer))
  (returns (`Amount Score` :type Integer))
  (bind _output_get (set `self.All Score` (+ (`KismetMathLibrary.Abs_Int` Score) (`self.All Score`))))
  (return _output_get))

(fn `GetCubesFoWin`
  (returns (AmountCubes :type Integer))
  (return (`KismetArrayLibrary.Array_Length` (`self.CubeArray`))))

(fn `UserConstructionScript`
  (for _index (range (+ (`self.X`) 1))
    (for _index_2 (range (+ (`self.Y`) 1))
      (bind _returnvalue (`AddComponent|NODE_AddStaticMeshComponent-2` :`RelativeTransform` (`KismetMathLibrary.MakeTransform` (`KismetMathLibrary.MakeVector` (`KismetMathLibrary.Conv_IntToDouble` (* _index (`self.Padding`))) (`KismetMathLibrary.Conv_IntToDouble` (* _index_2 (`self.Padding`)))))))
      (`KismetArrayLibrary.Array_Add` (`self.PreviewArray`) _returnvalue))))