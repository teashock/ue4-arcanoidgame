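; BP_Cube_Child is a child cube Blueprint for a hittable block that can drop a random actor when destroyed.
; BeginPlay binds its destroyed event, which has a 25% chance to spawn a random pick from the Class array at the Box location.
; The parent BeginPlay call runs only after that spawn, not at BeginPlay.
; HitBlock turns the cube red before running the parent's hit logic.
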(event `self.ReceiveBeginPlay`
  (add `Actor.OnDestroyed` (delegate `DestroyedCubes`)))

(event `DestroyedCubes`
  (params (DestroyedActor :type "Actor Object Reference"))
  (if (`KismetMathLibrary.RandomBoolWithWeight` 0.25)
    (`|SpawnActorFromClass` (`KismetArrayLibrary.Array_Random` (`self.Class`)) (`KismetMathLibrary.MakeTransform` (`SceneComponent.K2_GetComponentLocation` (`self.Box`))) "Undefined" "OverrideRootScale" null null)
    (`parent.ReceiveBeginPlay`)))

(event `self.Hit Block`
  (`PrimitiveComponent.SetMaterial` (`self.Cube`) 0 "/AnimationSharing/AnimSharingRed.AnimSharingRed")
  (`parent.Hit Block`))

(fn `UserConstructionScript`
  (`parent.UserConstructionScript`))